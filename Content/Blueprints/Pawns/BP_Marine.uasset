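; BP_Marine is the player-controlled marine pawn, with world-axis movement and separately driven aim.
; BeginPlay adds the gameplay Enhanced Input mapping context, and IA_Walk feeds movement input with its X and Y swapped onto world axes.
; Every tick, UpdatePlayerAim converts two raw axis-key readings through atan2 into a yaw-only control rotation on player controller 0.
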(event Input|EnhancedActionEvents|EnhancedInputActionIA_Walk
  (params (ActionValue :type Vector%202D%20Structure) (ElapsedSeconds :type Float%20%28double-precision%29) (TriggeredSeconds :type Float%20%28double-precision%29) (InputAction :type Input%20Action%20Object%20Reference :default "/Game/InputEnhanced/InputActions/IA_Walk.IA_Walk"))
  (:Triggered
    (Pawn|Input|AddMovementInput (Math|Vector|MakeVector (.y ActionValue) (.x ActionValue) 0.0) 1.0 false)))

(event EventBeginPlay
  (Input|AddMappingContext (PlayerController|LocalPlayerSubsystems|GetEnhancedInputLocalPlayerSubsystem (Game|GetPlayerController 0)) "/Game/InputEnhanced/InputMappingContext/IMC_GamePlayContext.IMC_GamePlayContext" 0 "(bIgnoreAllPressedKeysUntilRelease=True,bForceImmediately=False,bNotifyUserSettings=False)"))

(event Collision|EventActorBeginOverlap
  (params (OtherActor :type Actor%20Object%20Reference)))

(event EventTick
  (params (DeltaSeconds :type Float%20%28single-precision%29))
  (CallFunction|UpdatePlayerAim))

(fn ConstructionScript)

(fn UpdatePlayerAim
  (Pawn|SetControlRotation (Game|GetPlayerController 0) (Math|Rotator|MakeRotator 0.0 0.0 (Class|KismetMathLibrary|DegAtan2 (Class|Actor|GetInputAxisKeyValue) (Class|Actor|GetInputAxisKeyValue)))))